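; BP_Target is a damageable target actor that is destroyed when its health runs out.
; On any damage it subtracts the amount from its Heal variable, which acts as health.
; When Heal reaches zero it prints a debug message and destroys itself after a short delay, and later hits are ignored.
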(event `self.ReceiveAnyDamage`
  (params (Damage :type "Float (single-precision)") (DamageType :type "DamageType Object Reference") (InstigatedBy :type "Controller Object Reference") (DamageCauser :type "Actor Object Reference"))
  (bind _heal (`self.Heal`))
  (if (> _heal 0.0)
    (set `self.Heal` (- _heal Damage))
    (if (<= (`self.Heal`) 0.0)
      (`KismetSystemLibrary.PrintString` "BP_Target Yok Oluyor")
      (`KismetSystemLibrary.Delay` 0.2)
      (`self.K2_DestroyActor`))))

(fn `UserConstructionScript`)